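; Finish-line trigger actor for the turtle game that decides what happens when a turtle reaches the victory zone.
; On overlap by BP_TurtlePlayer it disables player movement, shows WBP_WinMenu and switches to Game and UI input with the mouse cursor visible.
; Overlap by BP_TurtleAI only prints a debug message, with no lose handling.
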(event Collision|EventActorBeginOverlap
  (params (OtherActor :type Actor%20Object%20Reference))
  (bind _returnvalue (Game|GetPlayerController 0))
  (Utilities|Casting|CastToBP_TurtlePlayer OtherActor
    (:then
      (Development|PrintString "You WIn!")
      (Pawn|Components|CharacterMovement|DisableMovement (Variables|/Script/Engine.Character|GetCharacterMovement (Game|GetPlayerCharacter 0)))
      (bind _returnvalue_2 (UserInterface|CreateWidget "/Game/UI/WBP_WinMenu.WBP_WinMenu_C" _returnvalue))
      (UserInterface|Viewport|AddtoViewport _returnvalue_2 0)
      (Input|SetInputModeGameandUI _returnvalue _returnvalue_2 "DoNotLock" true false)
      (Variables|/Script/Engine.PlayerController|SetbShowMouseCursor _returnvalue true))
    (:CastFailed
      (Utilities|Casting|CastToBP_TurtleAI OtherActor)
      (Development|PrintString "Turtle AI made it to victory zone "))))

(fn ConstructionScript)
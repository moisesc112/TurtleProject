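; BP_SandTrap is a one-shot enemy trap that spawns a crab when the turtle player character enters its trigger sphere.
; On overlap it rotates to face the player horizontally, then spawns BP_CrabEnemy at its transform, passing a crab mode, the player direction and its EmergeStart/EmergeEnd world locations.
; It then destroys itself; the OnTrapActivated and collision-disabling calls on the crab are unwired.
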(event OnComponentBeginOverlap(TriggerSphere)
  (params (OverlappedComponent :type Primitive%20Component%20Object%20Reference) (OtherActor :type Actor%20Object%20Reference) (OtherComp :type Primitive%20Component%20Object%20Reference) (OtherBodyIndex :type Integer) (bFromSweep :type Boolean) (SweepResult :type Hit%20Result%20Structure%20%28by%20ref%29))
  (bind _asbp_turtle_project_character (Utilities|Casting|CastToBP_TurtleProjectCharacter OtherActor))
  (bind _output_get (Variables|Default|SetPlayerDirection (Math|Vector|Normalize (Math|Vector|MakeVector (.X (Math|Vector|BreakVector (- (Math|Transform|TransformLocation (Transformation|GetActorTransform _asbp_turtle_project_character) "0, 0, 0") (Math|Transform|TransformLocation (Transformation|GetActorTransform) "0, 0, 0")))) (.Y (Math|Vector|BreakVector (- (Math|Transform|TransformLocation (Transformation|GetActorTransform _asbp_turtle_project_character) "0, 0, 0") (Math|Transform|TransformLocation (Transformation|GetActorTransform) "0, 0, 0")))) 0.0))))
  (Transformation|SetActorRotation (Math|Rotator|MakeRotfromX _output_get))
  (Development|PrintString "Overlapped with Sandtrap")
  (bind _returnvalue (Game|SpawnActorfromClass "/Game/Characters/Enemies/CrabEnemy/BP_CrabEnemy.BP_CrabEnemy_C" (Transformation|GetActorTransform) "Undefined" "MultiplyWithRoot" 0 "NewEnumerator1" _output_get (Transformation|GetWorldLocation (Variables|Default|GetEmergeStart)) (Transformation|GetWorldLocation (Variables|Default|GetEmergeEnd)) 0))
  (Actor|DestroyActor self))

(fn ConstructionScript)
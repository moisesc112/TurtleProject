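; Crab enemy character that emerges from and retracts to a hidden position, flagging aggro while the turtle player is within its detection range.
; One timeline lerps the actor between start and end points, playing forward to emerge and in reverse to retract.
; An EmergePhase value selects which completion event goes to the StateTree when the timeline finishes.
; The trap and patrol hooks are empty stubs.
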(event OnComponentBeginOverlap(DetectionRange)
  (params (OverlappedComponent :type Primitive%20Component%20Object%20Reference) (OtherActor :type Actor%20Object%20Reference) (OtherComp :type Primitive%20Component%20Object%20Reference) (OtherBodyIndex :type Integer) (bFromSweep :type Boolean) (SweepResult :type Hit%20Result%20Structure%20%28by%20ref%29))
  (Utilities|Casting|CastToTurtleProjectCharacter OtherActor)
  (Variables|Default|SetbInAggro true))

(event OnComponentEndOverlap(DetectionRange)
  (params (OverlappedComponent :type Primitive%20Component%20Object%20Reference) (OtherActor :type Actor%20Object%20Reference) (OtherComp :type Primitive%20Component%20Object%20Reference) (OtherBodyIndex :type Integer))
  (Utilities|Casting|CastToTurtleProjectCharacter OtherActor)
  (Variables|Default|SetbInAggro false))

(event Custom|OnTrapActivated)

(event Custom|OnStartEmerge
  (bind _output_get (Variables|Default|SetEmergePhase "NewEnumerator1"))
  (Transformation|SetRelativeRotation (Variables|Default|GetChildActor) "0.000000,90.000000,20.000000" false false)
  (bind _alpha (Timeline|Emerge%20Timeline PlayFromStart)
    (:Update
      (Transformation|SetActorLocation (Math|Vector|Lerp(Vector) (Variables|Default|GetEmergeStart) (Variables|Default|GetEmergeEnd) _alpha) false false))
    (:Finished
      (switch Utilities|FlowControl|Switch|SwitchonE_EmergePhase _output_get
        (:NewEnumerator1
          (Gameplay|StateTree|SendStateTreeEvent (Variables|Default|GetStateTree) (Utilities|Struct|MakeStateTreeEvent "(TagName=\"StateTree.Event.EmergingDone\")") :!class /Script/GameplayStateTreeModule.StateTreeComponent))
        (:NewEnumerator2
          (Gameplay|StateTree|SendStateTreeEvent (Variables|Default|GetStateTree) (Utilities|Struct|MakeStateTreeEvent "(TagName=\"StateTree.Event.RetractingDone\")") :!class /Script/GameplayStateTreeModule.StateTreeComponent))))))

(event Custom|OnStartRetract
  (Variables|Default|SetEmergePhase "NewEnumerator2")
  (bind _alpha (Timeline|Emerge%20Timeline ReverseFromEnd)
    (:Update
      (Transformation|SetActorLocation (Math|Vector|Lerp(Vector) (Variables|Default|GetEmergeStart) (Variables|Default|GetEmergeEnd) _alpha) false false))
    (:Finished
      (switch Utilities|FlowControl|Switch|SwitchonE_EmergePhase (stale Custom|OnStartEmerge _output_get)
        (:NewEnumerator1
          (Gameplay|StateTree|SendStateTreeEvent (Variables|Default|GetStateTree) (Utilities|Struct|MakeStateTreeEvent "(TagName=\"StateTree.Event.EmergingDone\")") :!class /Script/GameplayStateTreeModule.StateTreeComponent))
        (:NewEnumerator2
          (Gameplay|StateTree|SendStateTreeEvent (Variables|Default|GetStateTree) (Utilities|Struct|MakeStateTreeEvent "(TagName=\"StateTree.Event.RetractingDone\")") :!class /Script/GameplayStateTreeModule.StateTreeComponent))))))

(event EventBeginPlay
  (bind _asbp_crab_aicontroller (Utilities|Casting|CastToBP_CrabAIController (Pawn|GetController)))
  (Variables|Default|SetAIController _asbp_crab_aicontroller))

(event EventTick
  (params (DeltaSeconds :type Float%20%28single-precision%29))
  (Variables|Default|SetDeltaTime DeltaSeconds))

(fn ConstructionScript)

(fn EnterPatrolState)
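; Crab enemy that detects turtle characters, attacks and grabs them in its claw.
; A State Tree receives events as emerge, retract and player break-free finish, with emerging played as a montage and retracting as a reversed timeline.
; A timed sphere trace between claw sockets attaches the hit turtle, disabling player movement or AI logic and starting periodic damage.
; In one crab mode, Tick tilts the mesh to the floor normal outside attacks.
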(event OnComponentBeginOverlap(DetectionRange)
  (params (OverlappedComponent :type Primitive%20Component%20Object%20Reference) (OtherActor :type Actor%20Object%20Reference) (OtherComp :type Primitive%20Component%20Object%20Reference) (OtherBodyIndex :type Integer) (bFromSweep :type Boolean) (SweepResult :type Hit%20Result%20Structure%20%28by%20ref%29))
  (bind _asturtle_project_character (Utilities|Casting|CastToTurtleProjectCharacter OtherActor))
  (Variables|Default|SetbInAggro true)
  (Variables|Default|SetCurrentTarget _asturtle_project_character))

(event OnComponentBeginOverlap(HitBox)
  (params (OverlappedComponent :type Primitive%20Component%20Object%20Reference) (OtherActor :type Actor%20Object%20Reference) (OtherComp :type Primitive%20Component%20Object%20Reference) (OtherBodyIndex :type Integer) (bFromSweep :type Boolean) (SweepResult :type Hit%20Result%20Structure%20%28by%20ref%29)))

(event OnComponentEndOverlap(DetectionRange)
  (params (OverlappedComponent :type Primitive%20Component%20Object%20Reference) (OtherActor :type Actor%20Object%20Reference) (OtherComp :type Primitive%20Component%20Object%20Reference) (OtherBodyIndex :type Integer))
  (Utilities|Casting|CastToTurtleProjectCharacter OtherActor)
  (Variables|Default|SetbInAggro false)
  (Variables|Default|SetCurrentTarget 0))

(event Custom|OnTrapActivated)

(event Custom|OnStartEmerge
  (bind _output_get (Variables|Default|SetEmergePhase "NewEnumerator1"))
  (Animation|Montage|PlayMontage (Variables|Character|GetMesh) "/Game/Characters/Enemies/CrabEnemy/Animations/CrabAttack_Montage.CrabAttack_Montage"
    (:OnCompleted
      (switch Utilities|FlowControl|Switch|SwitchonE_EmergePhase _output_get
        (:NewEnumerator1
          (Gameplay|StateTree|SendStateTreeEvent (Variables|Default|GetStateTree) (Utilities|Struct|MakeStateTreeEvent "(TagName=\"StateTree.Event.EmergingDone\")") :!class /Script/GameplayStateTreeModule.StateTreeComponent))
        (:NewEnumerator2
          (if (Variables|Default|GetbHasPlayerGrabbed)
            (Development|PrintString "Sending Grabbed")
            (Gameplay|StateTree|SendStateTreeEvent (Variables|Default|GetStateTree) (Utilities|Struct|MakeStateTreeEvent "(TagName=\"StateTree.Event.RetractingDoneGrabbed\")") :!class /Script/GameplayStateTreeModule.StateTreeComponent)
            (else
              (Development|PrintString "Sending Retract")
              (Gameplay|StateTree|SendStateTreeEvent (Variables|Default|GetStateTree) (Utilities|Struct|MakeStateTreeEvent "(TagName=\"StateTree.Event.RetractingDone\")") :!class /Script/GameplayStateTreeModule.StateTreeComponent))))))))

(event Custom|OnStartRetract
  (Variables|Default|SetEmergePhase "NewEnumerator2")
  (bind _alpha (Timeline|Emerge%20Timeline ReverseFromEnd)
    (:Update
      (Transformation|SetActorLocation (Math|Vector|Lerp(Vector) (Variables|Default|GetLaunchStart) (Variables|Default|GetEmergeEnd) _alpha) false false))
    (:Finished
      (switch Utilities|FlowControl|Switch|SwitchonE_EmergePhase (stale Custom|OnStartEmerge _output_get)
        (:NewEnumerator1
          (Gameplay|StateTree|SendStateTreeEvent (Variables|Default|GetStateTree) (Utilities|Struct|MakeStateTreeEvent "(TagName=\"StateTree.Event.EmergingDone\")") :!class /Script/GameplayStateTreeModule.StateTreeComponent))
        (:NewEnumerator2
          (if (Variables|Default|GetbHasPlayerGrabbed)
            (Development|PrintString "Sending Grabbed")
            (Gameplay|StateTree|SendStateTreeEvent (Variables|Default|GetStateTree) (Utilities|Struct|MakeStateTreeEvent "(TagName=\"StateTree.Event.RetractingDoneGrabbed\")") :!class /Script/GameplayStateTreeModule.StateTreeComponent)
            (else
              (Development|PrintString "Sending Retract")
              (Gameplay|StateTree|SendStateTreeEvent (Variables|Default|GetStateTree) (Utilities|Struct|MakeStateTreeEvent "(TagName=\"StateTree.Event.RetractingDone\")") :!class /Script/GameplayStateTreeModule.StateTreeComponent))))))))

(event Custom|AttackTrace
  (bind _mesh (Variables|Character|GetMesh))
  (bind _mesh_2 (Variables|Character|GetMesh))
  (bind _returnvalue (Transformation|GetSocketTransform _mesh "cutterclaw_RSocket" "RTS_Component"))
  (bind (_outhit _returnvalue_2) (Collision|SphereTraceForObjects (.location (Transformation|GetSocketTransform _mesh_2 "cutterclaw_LSocket" "RTS_World")) (.location (Transformation|GetSocketTransform _mesh_2 "cutterclaw_RSocket" "RTS_World")) 4e+01 (Utilities|Array|MakeArray "ObjectTypeQuery3") false 0 "ForDuration" true "(R=1.000000,G=0.000000,B=0.000000,A=1.000000)" "(R=0.000000,G=1.000000,B=0.000000,A=1.000000)" 0.1))
  (if _returnvalue_2
    (Default|StopAttackTrace self)
    (Development|PrintString (Utilities|GetDisplayName (.HitActor (Collision|BreakHitResult _outhit))))
    (bind _output_get (Variables|Default|SetGrabbedTarget (.HitActor (Collision|BreakHitResult _outhit))))
    (Variables|Default|SetbHasPlayerGrabbed true)
    (bind _asbp_turtle_base (Utilities|Casting|CastToBP_TurtleBase _output_get))
    (Collision|SetCollisionEnabled (Variables|/Script/Engine.Character|GetCapsuleComponent _asbp_turtle_base) "NoCollision")
    (Collision|SetCollisionResponsetoChannel (Variables|/Script/Engine.Character|GetCapsuleComponent _asbp_turtle_base) "ECC_Pawn" "ECR_Ignore")
    (if (Pawn|IsPlayerControlled _asbp_turtle_base)
      (Pawn|Components|CharacterMovement|DisableMovement (Variables|/Script/Engine.Character|GetCharacterMovement _asbp_turtle_base))
      (else
        (bind _asbp_turtle_ai (Utilities|Casting|CastToBP_TurtleAI _asbp_turtle_base))
        (AI|Logic|StopLogic (Variables|/Game/Characters/Player/Blueprints/BP_TurtleAI.BP_TurtleAI_C|GetStateTree _asbp_turtle_ai) "")))
    (Transformation|AttachComponentToComponent _asbp_turtle_base (Variables|Character|GetMesh) "cutterclaw_tip_RSocket" "SnapToTarget" "KeepWorld" "KeepWorld" false)
    (bind _asbp_turtle_base_2 (Utilities|Casting|CastToBP_TurtleBase (Variables|Default|GetGrabbedTarget)))
    (if (Pawn|IsPlayerControlled _asbp_turtle_base_2)
      (Class|BPIGrabbable|OnGrabbed(Message) _asbp_turtle_base_2 self))
    (Default|StartPeriodicDamage _asbp_turtle_base_2)
    (Transformation|SetWorldRotation (Variables|/Script/Engine.Character|GetMesh _asbp_turtle_base_2) (Math|Rotator|MakeRotator (* (.pitch (.rotation _returnvalue)) -1.0) 0.0 (+ (.yaw (.rotation _returnvalue)) 0.0)) false false)))

(event EventBeginPlay
  (bind _asbp_crab_aicontroller (Utilities|Casting|CastToBP_CrabAIController (Pawn|GetController)))
  (Variables|Default|SetAIController _asbp_crab_aicontroller)
  (Variables|Default|SetBaseMeshRot (.Rotation (Math|Transform|BreakTransform (Transformation|GetRelativeTransform (Variables|Character|GetMesh))))))

(event EventOnReleasePlayer
  (if (Variables|Default|GetbCanPlayerBreakFree)
    (Variables|Default|SetbHasPlayerGrabbed false)
    (Gameplay|StateTree|SendStateTreeEvent (Variables|Default|GetStateTree) (Utilities|Struct|MakeStateTreeEvent "(TagName=\"StateTree.Event.PlayerJump\")") :!class /Script/GameplayStateTreeModule.StateTreeComponent)
    (Variables|Default|SetbCanPlayerBreakFree false)))

(event EventTick
  (params (DeltaSeconds :type Float%20%28single-precision%29))
  (Variables|Default|SetDeltaTime DeltaSeconds)
  (if (== (Variables|Default|GetCrabMode) 0)
    (if (not (Variables|Default|GetbInAttackMontage))
      (bind (_bisgrounded _impactnormal) (CallFunction|GetImpactNormal))
      (CallFunction|UpdateMeshRotation _bisgrounded _impactnormal))))

(event EventStartAttackTrace
  (bind _returnvalue (Utilities|Time|SetTimerbyEvent (delegate Custom|AttackTrace) 0.05 true))
  (Variables|Default|SetAttackTraceLoop _returnvalue)
  (Variables|Default|SetbInAttackMontage true))

(event EventStopAttackTrace
  (bind _attacktraceloop (Variables|Default|GetAttackTraceLoop))
  (if (Utilities|Time|IsValidTimerHandle _attacktraceloop)
    (Utilities|Time|ClearandInvalidateTimerbyHandle _attacktraceloop)
    (Variables|Default|SetbInAttackMontage false)))

(fn ConstructionScript)

(fn EnterPatrolState)

(fn UpdateMeshRotation
  (params (bIsGrounded :type Boolean) (ImpactNormal :type Vector))
  (bind _returnvalue (Transformation|GetActorForwardVector))
  (bind _returnvalue_2 (Math|Vector|ProjectVectorontoPlane _returnvalue ImpactNormal))
  (bind _returnvalue_3 (Math|Rotator|MakeRotfromZX ImpactNormal _returnvalue_2))
  (bind (_roll _pitch) (Math|Rotator|BreakRotator _returnvalue_3))
  (bind _output_get (LocalVariables|SetCurrentTilt (Math|Interpolation|RInterpTo (LocalVariables|GetCurrentTilt) (Math|Rotator|MakeRotator _roll _pitch 0.0) (Variables|Default|GetDeltaTime) (LocalVariables|GetMovementChangeRate))))
  (Transformation|SetRelativeRotation (Variables|Character|GetMesh) (Math|Rotator|CombineRotators (Variables|Default|GetBaseMeshRot) _output_get) false false))

(fn GetImpactNormal
  (bind _charactermovement (Variables|Character|GetCharacterMovement))
  (bind _currentfloor (Variables|/Script/Engine.CharacterMovementComponent|GetCurrentFloor _charactermovement))
  (bind (_bblockinghit _bwalkablefloor _blinetrace _floordist _linedist _hitresult) (Utilities|Struct|BreakFindFloorResult _currentfloor))
  (if _bwalkablefloor
    (return true (.ImpactNormal (Collision|BreakHitResult _hitresult)))
    (else
      (return false "0, 0, 0"))))
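; Bird enemy that waits for the player to enter its trigger sphere, apparently to perform a shadowed sweep attack.
; On entry it disables the trigger, enables capsule overlaps, shows the shadow and sends PlayerInBirdTrigger to its StateTree.
; Capsule overlaps only print hit or miss.
; An unwired timeline holds a sweep that moves bird and shadow, then sphere-checks to damage and attach the player to DragAnchor.
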(event OnComponentBeginOverlap(TriggerSphere)
  (params (OverlappedComponent :type Primitive%20Component%20Object%20Reference) (OtherActor :type Actor%20Object%20Reference) (OtherComp :type Primitive%20Component%20Object%20Reference) (OtherBodyIndex :type Integer) (bFromSweep :type Boolean) (SweepResult :type Hit%20Result%20Structure%20%28by%20ref%29))
  (if (== OtherActor (Game|GetPlayerCharacter 0))
    (Variables|/Script/Engine.PrimitiveComponent|SetbGenerateOverlapEvents (Variables|Default|GetTriggerSphere) false)
    (Variables|Default|SetBirdShadowScale (Variables|/Script/Engine.SceneComponent|GetRelativeScale3D (Variables|Default|GetBirdShadow)))
    (Variables|Default|SetCapsuleScale (Variables|/Script/Engine.SceneComponent|GetRelativeScale3D (Variables|Default|GetCapsule)))
    (Variables|/Script/Engine.PrimitiveComponent|SetbGenerateOverlapEvents (Variables|Default|GetCapsule) true)
    (Rendering|SetVisibility (Variables|Default|GetBirdShadow) true false)
    (Gameplay|StateTree|SendStateTreeEvent (Variables|Default|GetStateTree) (Utilities|Struct|MakeStateTreeEvent "(TagName=\"StateTree.Event.PlayerInBirdTrigger\")") :!class /Script/GameplayStateTreeModule.StateTreeComponent)))

(event OnComponentBeginOverlap(Capsule)
  (params (OverlappedComponent :type Primitive%20Component%20Object%20Reference) (OtherActor :type Actor%20Object%20Reference) (OtherComp :type Primitive%20Component%20Object%20Reference) (OtherBodyIndex :type Integer) (bFromSweep :type Boolean) (SweepResult :type Hit%20Result%20Structure%20%28by%20ref%29))
  (if (== (Game|GetPlayerCharacter 0) OtherActor)
    (Development|PrintString "bird hit player")
    (else
      (Development|PrintString "bird missed player"))))

(event EventBeginPlay
  (Variables|Default|SetDistanceBtwnMeshNShadow (- (Transformation|GetWorldLocation (Variables|Default|GetSkeletalMesh)) (Transformation|GetWorldLocation (Variables|Default|GetBirdShadow)))))

(fn ConstructionScript)
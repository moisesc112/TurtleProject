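; Bird enemy that makes a single telegraphed strike on the turtle player character.
; An overlap on its trigger sphere disables further overlaps, then reveals the bird shadow and grows it on a timeline as a warning.
; When the timeline finishes, a debug-drawn sphere query, offset along Y by the trigger radius, checks for pawns.
; If the player is caught, it applies a damage instance and destroys itself.
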(event OnComponentBeginOverlap(TriggerSphere)
  (params (OverlappedComponent :type Primitive%20Component%20Object%20Reference) (OtherActor :type Actor%20Object%20Reference) (OtherComp :type Primitive%20Component%20Object%20Reference) (OtherBodyIndex :type Integer) (bFromSweep :type Boolean) (SweepResult :type Hit%20Result%20Structure%20%28by%20ref%29))
  (bind _triggersphere (Variables|Default|GetTriggerSphere))
  (bind _triggersphere_2 (Variables|Default|GetTriggerSphere))
  (bind _returnvalue (Transformation|GetWorldLocation _triggersphere))
  (bind _returnvalue_2 (Components|Sphere|GetScaledSphereRadius _triggersphere_2))
  (bind _returnvalue_3 (Math|Vector|MakeVector 0.0 _returnvalue_2 0.0))
  (bind _returnvalue_4 (+ _returnvalue _returnvalue_3))
  (Variables|/Script/Engine.PrimitiveComponent|SetbGenerateOverlapEvents (Variables|Default|GetTriggerSphere) false)
  (Variables|Default|SetBirdShadowScale (Variables|/Script/Engine.SceneComponent|GetRelativeScale3D (Variables|Default|GetBirdShadow)))
  (Rendering|SetVisibility (Variables|Default|GetBirdShadow) true false)
  (bind _shadowscaletrack (Timeline|Shadow%20Scale%20Timeline PlayFromStart)
    (:Update
      (Transformation|SetRelativeScale3D (Variables|Default|GetBirdShadow) (Math|Vector|Lerp(Vector) (Variables|Default|GetBirdShadowScale) (Math|Vector|MakeVector 3.0 3.0 3.0) _shadowscaletrack)))
    (:Finished
      (Rendering|Debug|DrawDebugSphere _returnvalue_4 4e+02 12 "(R=1.000000,G=0.010696,B=0.989103,A=1.000000)" 5.0)
      (bind (_outactors _returnvalue_5) (Collision|SphereOverlapActors _returnvalue_4 4e+02 (Utilities|Array|MakeArray "ObjectTypeQuery3") 0))
      (for _array_element _outactors
        (if (== _array_element (Game|GetPlayerCharacter 0))
          (Development|PrintString "Turtle overlap in bird" _returnvalue_5)
          (bind _asbp_turtle_project_character (Utilities|Casting|CastToBP_TurtleProjectCharacter (Game|GetPlayerCharacter 0)))
          (Default|ApplyDamageInstance _asbp_turtle_project_character)
          (Actor|DestroyActor)
          (else
            (Development|PrintString "not player")))))))

(fn ConstructionScript)
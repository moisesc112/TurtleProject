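; BP_BirdManager is a pool manager for sweeping bird enemies.
; On BeginPlay it spawns one BP_BirdEnemySweep per pool slot at its matching spawn point, passing that point as the patrol start.
; RequestBird hands out the first available bird and marks it busy, while ReturnBird marks it available again.
; An older timer-driven staggered spawn with a hard-coded location remains in the graph but never runs.
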(event Custom|SpawnNextBird)

(event EventBeginPlay
  (for _index (range 0 (- (Variables|Default|GetPoolSize) 1))
    (bind _returnvalue (Game|SpawnActorfromClass "/Game/Characters/Enemies/BirdEnemy/Blueprints/BP_BirdEnemySweep.BP_BirdEnemySweep_C" (Math|Conversions|ToTransform(Vector) (Utilities|Array|Get(acopy) (Variables|Default|GetSpawnPoints) _index)) "Undefined" "MultiplyWithRoot" 0 (Utilities|Array|Get(acopy) (Variables|Default|GetSpawnPoints) _index) 0))
    (Utilities|Array|Add (Variables|Default|GetBirdPool) _returnvalue)))

(event EventTick
  (params (DeltaSeconds :type Float%20%28single-precision%29)))

(fn ConstructionScript)

(fn RequestBird
  (for _array_element (Variables|Default|GetBirdPool)
    (if (Variables|/Game/Characters/Enemies/BirdEnemy/Blueprints/BP_BirdEnemySweep.BP_BirdEnemySweep_C|GetbIsAvailable _array_element)
      (Variables|/Game/Characters/Enemies/BirdEnemy/Blueprints/BP_BirdEnemySweep.BP_BirdEnemySweep_C|SetbIsAvailable _array_element false)
      (return _array_element)))
  (return 0))

(fn ReturnBird
  (params (BirdEnemy :type BP%20Bird%20Enemy%20Sweep%20Object%20Reference))
  (Variables|/Game/Characters/Enemies/BirdEnemy/Blueprints/BP_BirdEnemySweep.BP_BirdEnemySweep_C|SetbIsAvailable BirdEnemy true))
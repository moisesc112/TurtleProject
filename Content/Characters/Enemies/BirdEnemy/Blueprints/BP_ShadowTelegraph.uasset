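; BP_ShadowTelegraph is a bird enemy telegraph that shows a shadow decal under the turtle player.
; While tracking, Tick snaps its root to CurrentPlayer's location each frame and steadily grows the decal's Y and Z scale.
; BeginPlay waits TrackDuration, then stops tracking so the shadow stays in place, and clears HasShadow on the player's BP_TurtleBase.
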(event EventBeginPlay
  (Utilities|FlowControl|Delay (Variables|Default|GetTrackDuration))
  (Variables|Default|SetbTrackingPlayer false)
  (bind _asbp_turtle_project_character (Utilities|Casting|CastToBP_TurtleBase (Variables|Default|GetCurrentPlayer)))
  (Variables|/Game/Characters/Player/Blueprints/BP_TurtleBase.BP_TurtleBase_C|SetbHasShadow _asbp_turtle_project_character false))

(event EventTick
  (params (DeltaSeconds :type Float%20%28single-precision%29))
  (bind _returnvalue (* DeltaSeconds 0.5))
  (if (Variables|Default|GetbTrackingPlayer)
    (Transformation|SetWorldLocation (Variables|Default|GetDefaultSceneRoot) (Transformation|GetActorLocation (Variables|Default|GetCurrentPlayer)) false false)
    (Transformation|SetWorldScale3D (Variables|Default|GetShadowDecal) (+ (Transformation|GetWorldScale (Variables|Default|GetShadowDecal)) (Math|Vector|MakeVector 0.0 _returnvalue _returnvalue)))))

(fn ConstructionScript)
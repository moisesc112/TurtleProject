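; BP_BirdActivation is a one-shot trigger zone that launches a bird enemy at the turtle player.
; When the turtle overlaps its sphere without already having a shadow, it sets HasShadow and spawns a BP_ShadowTelegraph at the turtle.
; It requests a bird from BP_BirdManager, activates it with the turtle and telegraph, then destroys itself.
; The CallOnZoneActivated dispatcher call is disconnected and never runs.
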(event OnComponentBeginOverlap(TriggerSphere)
  (params (OverlappedComponent :type Primitive%20Component%20Object%20Reference) (OtherActor :type Actor%20Object%20Reference) (OtherComp :type Primitive%20Component%20Object%20Reference) (OtherBodyIndex :type Integer) (bFromSweep :type Boolean) (SweepResult :type Hit%20Result%20Structure%20%28by%20ref%29))
  (bind _returnvalue (Actor|GetActorOfClass "/Game/Characters/Player/Blueprints/BP_TurtleBase.BP_TurtleBase_C"))
  (if (== _returnvalue OtherActor)
    (bind _asbp_turtle_project_character (Utilities|Casting|CastToBP_TurtleBase OtherActor))
    (if (Variables|/Game/Characters/Player/Blueprints/BP_TurtleBase.BP_TurtleBase_C|GetbHasShadow _asbp_turtle_project_character)
      (Development|PrintString "Turtle has shadow currently on it already")
      (else
        (bind _asbp_turtle_project_character_2 (Utilities|Casting|CastToBP_TurtleBase OtherActor))
        (Variables|/Game/Characters/Player/Blueprints/BP_TurtleBase.BP_TurtleBase_C|SetbHasShadow _asbp_turtle_project_character_2 true)
        (bind _returnvalue_2 (Game|SpawnActorfromClass "/Game/Characters/Enemies/BirdEnemy/Blueprints/BP_ShadowTelegraph.BP_ShadowTelegraph_C" (Math|Transform|MakeTransform (Transformation|GetActorLocation _asbp_turtle_project_character_2) (Transformation|GetActorRotation _asbp_turtle_project_character_2)) "Undefined" "MultiplyWithRoot" 0 _asbp_turtle_project_character_2 0))
        (bind _birdenemy (Default|RequestBird (Variables|Default|GetBirdManager)))
        (Default|OnTriggerActivated _birdenemy _asbp_turtle_project_character_2 _returnvalue_2)
        (Actor|DestroyActor)))))

(event EventBeginPlay
  (bind _returnvalue (Actor|GetActorOfClass "/Game/Characters/Enemies/BirdEnemy/Blueprints/BP_BirdManager.BP_BirdManager_C"))
  (Variables|Default|SetBirdManager _returnvalue))

(fn ConstructionScript)
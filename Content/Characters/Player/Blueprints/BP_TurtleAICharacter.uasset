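; BP_TurtleAICharacter is an AI-controlled turtle character Blueprint that chases the player.
; On BeginPlay it issues a single AI MoveTo toward the player character with a near-zero acceptance radius, printing a message if the move fails.
; Each tick it shows the current value of its stamina component on screen as debug text, alongside calls to parent logic.
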(event EventBeginPlay
  (|CallParentFunction)
  (AI|AIMoveTo self "0, 0, 0" (Game|GetPlayerCharacter 0) 0.0001 false
    (:OnFail
      (Development|PrintString "ai turtle movement failed"))))

(event Collision|EventActorBeginOverlap
  (params (OtherActor :type Actor%20Object%20Reference)))

(event EventTick
  (params (DeltaSeconds :type Float%20%28single-precision%29))
  (|CallParentFunction DeltaSeconds)
  (Development|PrintText (Utilities|Text|FormatText "AI Current Stamina: {Stamina}" (Class|TurtleStaminaComponent|GetCurrentStamina (Variables|Default|GetBP_StaminaComponent))) true false))

(fn ConstructionScript
  (|CallParentFunction))
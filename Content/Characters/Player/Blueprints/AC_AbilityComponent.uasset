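; Player ability component that decides whether a dash can happen and computes the resulting velocity.
; TryDash reads current stamina from the passed-in stamina component and allows the dash while it is above zero.
; It then adds the flattened, normalized dash direction scaled by DashStrength to the current velocity, leaving the caller to apply it.
; Stamina is only checked, never consumed, and a failed dash prints a debug message.
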(event EventBeginPlay)

(event EventTick
  (params (DeltaSeconds :type Float%20%28single-precision%29)))

(fn HasEnoughStamina
  (params (CurrentStamina :type Float%20%28double-precision%29))
  (return (> CurrentStamina 0.0)))

(fn TryDash
  (params (CurrentVelocity :type Vector) (DashDirection :type Vector) (StaminaComponent :type BP%20Stamina%20Component%20Object%20Reference))
  (bind (_x _y) (Math|Vector|BreakVector DashDirection))
  (bind _bcanuseability (CallFunction|HasEnoughStamina (Class|TurtleStaminaComponent|GetCurrentStamina StaminaComponent)))
  (if _bcanuseability
    (return (+ CurrentVelocity (* (Math|Vector|Normalize (Math|Vector|MakeVector _x _y 0.0)) (LocalVariables|GetDashStrength))) true)
    (else
      (Development|PrintString "Not Enough Stamina to Dash")
      (return "0, 0, 0" false))))
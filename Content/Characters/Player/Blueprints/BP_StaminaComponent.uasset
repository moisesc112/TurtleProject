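; Player stamina component that tracks current stamina for sprinting and jumping, starting at maximum on BeginPlay.
; DrainStamina subtracts a jump cost or a rate-based amount and RegenStamina adds it back, both capping at maximum minus DamageTaken.
; CanSprint reports whether stamina remains.
; Tick calls DrainStamina while sprinting but passes zero DeltaTime, so that call subtracts nothing, and nothing here calls RegenStamina.
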(event EventBeginPlay
  (CallFunction|SetStamina (Variables|Default|GetMaxStamina)))

(event EventTick
  (params (DeltaSeconds :type Float%20%28single-precision%29))
  (if (Variables|Default|GetbIsSprinting)
    (CallFunction|DrainStamina 0.0 0.0 false)))

(fn DrainStamina
  (params (Delta%20Time :type Float%20%28double-precision%29) (DamageTaken :type Float%20%28double-precision%29) (JustJumped :type Boolean))
  (if JustJumped
    (Variables|Default|SetCurrentStamina (Math|Float|Clamp(Float) (- (Variables|Default|GetCurrentStamina) (LocalVariables|GetJumpStaminaUsage)) 0.0 (- (Variables|Default|GetMaxStamina) DamageTaken)))
    (else
      (Variables|Default|SetCurrentStamina (Math|Float|Clamp(Float) (- (Variables|Default|GetCurrentStamina) (* Delta%20Time (Variables|Default|GetDrainRate))) 0.0 (- (Variables|Default|GetMaxStamina) DamageTaken))))))

(fn GetStamina
  (return (Variables|Default|GetCurrentStamina)))

(fn CanSprint
  (return (> (Variables|Default|GetCurrentStamina) 0.0)))

(fn SetSprinting
  (params (NewIsSprinting :type Boolean))
  (Variables|Default|SetbIsSprinting NewIsSprinting))

(fn SetStamina
  (params (New%20Stamina :type Float%20%28double-precision%29))
  (Variables|Default|SetCurrentStamina New%20Stamina))

(fn RegenStamina
  (params (DeltaTime :type Float%20%28double-precision%29) (DamageTaken :type Float%20%28double-precision%29))
  (Variables|Default|SetCurrentStamina (Math|Float|Clamp(Float) (+ (Variables|Default|GetCurrentStamina) (* DeltaTime (Variables|Default|GetRegenRate))) 0.0 (- (Variables|Default|GetMaxStamina) DamageTaken))))
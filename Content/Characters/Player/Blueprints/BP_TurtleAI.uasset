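; BP_TurtleAI is an AI-driven turtle character that uses a StateTree and a route of waypoints.
; On BeginPlay it gathers all BP_TurtleWayPoint actors, orders them by their Index, targets the first and starts the StateTree.
; Tick sends a one-time StateTree event when stamina runs out during a slide.
; Tick also draws a debug point trail and prints stamina, velocity, slide state and target waypoint.
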(event EventBeginPlay
  (|CallParentFunction)
  (bind _outactors (Actor|GetAllActorsOfClass "/Game/Gameplay/Blueprints/BP_TurtleWayPoint.BP_TurtleWayPoint_C"))
  (bind _output_get (Variables|Default|SetWaypoints _outactors))
  (for (_ _array_index) _output_get
    (for _array_element _output_get
      (if (== (Variables|/Game/Gameplay/Blueprints/BP_TurtleWayPoint.BP_TurtleWayPoint_C|GetIndex _array_element) _array_index)
        (Utilities|Array|Insert (Variables|Default|GetSortedWaypoints) _array_element _array_index))))
  (bind _output_get_2 (Variables|Default|SetTargetWaypoint (Utilities|Array|Get(acopy) (Variables|Default|GetSortedWaypoints))))
  (Development|PrintString (Utilities|GetDisplayName _output_get_2))
  (AI|Logic|StartLogic (Variables|Default|GetStateTree)))

(event Collision|EventActorBeginOverlap
  (params (OtherActor :type Actor%20Object%20Reference)))

(event EventTick
  (params (DeltaSeconds :type Float%20%28single-precision%29))
  (|CallParentFunction DeltaSeconds)
  (Rendering|Debug|DrawDebugPoint (Transformation|GetActorLocation self) 5.0 "(R=1.000000,G=0.034555,B=0.925658,A=1.000000)" 1e+04)
  (Development|PrintText (Utilities|Text|FormatText "AI Current Stamina: {Stamina}, Current Velocity: {Velocity}, Is Sliding: {IsSliding}, Waypoint: {Waypoint}" (Class|TurtleStaminaComponent|GetCurrentStamina (Variables|Default|GetStaminaComponent)) (|GenerictoText (Variables|/Script/Engine.MovementComponent|GetVelocity (Variables|Character|GetCharacterMovement))) (Variables|Default|GetbIsSliding) (Utilities|GetDisplayName (Variables|Default|GetTargetWaypoint))) true false)
  (if (not (Variables|Default|GetbHasSentEvent))
    (if (Variables|Default|GetbIsSliding)
      (if (<= (Class|TurtleStaminaComponent|GetCurrentStamina (Variables|Default|GetStaminaComponent)) 0.0)
        (Gameplay|StateTree|SendStateTreeEvent (Variables|Default|GetStateTree) (Utilities|Struct|MakeStateTreeEvent "(TagName=\"Test\")") :!class /Script/GameplayStateTreeModule.StateTreeComponent)
        (Variables|Default|SetbHasSentEvent true)))))

(fn ConstructionScript
  (|CallParentFunction))

(fn Die
  (|CallParentFunction))